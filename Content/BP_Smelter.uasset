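; Smelter building that turns requested input items into produced items through a Transformer component.
; On initialization and after each produced item, it requests every Transformer input from the ItemSink.
; Items arriving at the sink are added to the Inventory.
; Tick refreshes a text readout of transformer state, input stock, the outstanding request (hard-coded to IronOre) and output quantity.
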(event OnItemAdded(ItemSink)
  (params (Type :type Name :default "None") (Quantity :type Integer))
  (Class|InventoryComponent|Add (Variables|Default|GetInventory) Type Quantity))

(event OnInitializing(Transformer)
  (params (OldState :type ETransformerState%20Enum :default "Initializing"))
  (CallFunction|RequestInputs))

(event OnItemProduced(Transformer)
  (params (OldState :type ETransformerState%20Enum :default "Initializing"))
  (CallFunction|RequestInputs))

(event OnTransformingStarted(Transformer)
  (params (OldState :type ETransformerState%20Enum :default "Initializing")))

(event EventTick
  (params (DeltaSeconds :type Float%20%28single-precision%29))
  (bind _returnvalue (Class|ItemSinkComponent|GetItemsNeededforType (Variables|Default|GetItemSink) "IronOre"))
  (Rendering|Components|TextRender|SetText (Variables|Default|GetTextRender) (Utilities|Text|FormatText "{State}: {Inputs}/{Requested}, {Outputs}" (Utilities|String|EnumtoString (Variables|/Script/SimRTS.TransformerComponent|GetState (Variables|Default|GetTransformer))) (CallFunction|GetInputsDescription) _returnvalue (Variables|/Script/SimRTS.ItemSourceComponent|GetQuantity (Variables|Default|GetOutput)))))

(fn ConstructionScript)

(fn RequestInputs
  (for _array_element (Variables|/Script/SimRTS.TransformerComponent|GetInputs (Variables|Default|GetTransformer))
    (Class|ItemSinkComponent|AddRequestforType (Variables|Default|GetItemSink) (.type _array_element) (.quantity _array_element))))

(fn GetInputsDescription
  (for _array_element (Variables|/Script/SimRTS.TransformerComponent|GetInputs (Variables|Default|GetTransformer))
    (LocalVariables|SetOutput (Utilities|String|ToString(Text) (Utilities|Text|FormatText "{Prev}{Type}: {Quantity}/{Max} 
" (LocalVariables|GetOutput) (.type _array_element) (Class|InventoryComponent|GetQuantity (Variables|Default|GetInventory) (.type _array_element)) (.quantity _array_element)))))
  (return (LocalVariables|GetOutput)))